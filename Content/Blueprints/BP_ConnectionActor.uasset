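; Lobby actor that reveals a mesh and name label representing a player who has logged in.
; BeginPlay applies the current visibility flag to the static mesh and name widget.
; OnPlayerLogIn activates a Niagara effect, shows both, writes the PlayerState name into W_LobbyPlayerWidget and stores the flag and name.
; RepNotifies on those two variables mirror visibility and name text on clients.
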(event Custom|OnPlayerLogIn
  (params (PlayerState :type Player%20State%20Object%20Reference))
  (bind _returnvalue (PlayerState|GetPlayerName PlayerState))
  (bind _nameplayer (Variables|Default|GetNamePlayer))
  (bind _niagara (Variables|Default|GetNiagara))
  (bind _returnvalue_2 (UserInterface|GetWidget _nameplayer))
  (Components|Activation|Activate _niagara false)
  (Animation|GetPlayLength _niagara)
  (Rendering|SetVisibility (Variables|Default|GetStaticMesh) true false)
  (Variables|Default|SetNeedToBeVisible true)
  (Widget|SetVisibility _returnvalue_2 "Visible")
  (bind _asw_lobby_player_widget (Utilities|Casting|CastToW_LobbyPlayerWidget _returnvalue_2))
  (Default|SetText _asw_lobby_player_widget (Utilities|Text|ToText(String) _returnvalue))
  (Variables|Default|SetNamePlayerStart _returnvalue))

(event EventBeginPlay
  (bind _needtobevisible (Variables|Default|GetNeedToBeVisible))
  (Rendering|SetVisibility (Variables|Default|GetStaticMesh) _needtobevisible false)
  (if _needtobevisible
    (Widget|SetVisibility (UserInterface|GetWidget (Variables|Default|GetNamePlayer)) "Visible")
    (else
      (Widget|SetVisibility (UserInterface|GetWidget (Variables|Default|GetNamePlayer)) "Collapsed"))))

(fn ConstructionScript)

(fn OnRepNeedtobeVisible
  (Rendering|SetVisibility (Variables|Default|GetStaticMesh) (Variables|Default|GetNeedToBeVisible) false)
  (if (Variables|Default|GetNeedToBeVisible)
    (Widget|SetVisibility (UserInterface|GetWidget (Variables|Default|GetNamePlayer)) "Visible")
    (else
      (Widget|SetVisibility (UserInterface|GetWidget (Variables|Default|GetNamePlayer)) "Collapsed"))))

(fn OnRepNamePlayerStart
  (bind _asw_lobby_player_widget (Utilities|Casting|CastToW_LobbyPlayerWidget (UserInterface|GetWidget (Variables|Default|GetNamePlayer))))
  (Default|SetText _asw_lobby_player_widget (Utilities|Text|ToText(String) (Variables|Default|GetNamePlayerStart))))

(fn OnRepNewVar)