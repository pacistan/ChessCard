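; Template card actor that shows a game card with a name widget, a sleeve and a spinning 3D unit piece.
; ConstructCard fills the widget name from row data and async-loads the piece's static mesh, which Tick rotates continuously.
; UpdateMaterials applies the sleeve materials mapped to the current card state.
; Discard, draw and play events trigger sounds, with variants for Gold-effect draws and movement plays.
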(event EventBeginPlay)

(event Collision|EventActorBeginOverlap
  (params (OtherActor :type Actor%20Object%20Reference)))

(event EventBPEonDiscardCard
  (Audio|PlaySoundatLocation (Variables|Default|GetSoundCue_Discard) (Transformation|GetActorLocation) "0, 0, 0" 1.0 1.0 0.0 0 0 0 0))

(event EventConstructCard
  (params (RowHandle :type Card%20Data%20Structure))
  (bind _asw_card_widget (Utilities|Casting|CastToW_CardWidget (UserInterface|GetWidget (Variables|Default|GetCardWidget))))
  (Default|ChangeCardName _asw_card_widget (Utilities|String|StringToName (.cardname RowHandle)))
  (bind _object (Utilities|AsyncLoadAsset (.cardunitstaticmesh RowHandle))
    (:Completed
      (bind _asstatic_mesh (Utilities|Casting|CastToStaticMesh _object))
      (Components|StaticMesh|SetStaticMesh (Variables|Default|GetPiece_Mesh) _asstatic_mesh))))

(event EventUpdateMaterials
  (bind _materialmap (Variables|Default|GetMaterialMap))
  (bind _currentcardstate (Variables|Default|GetCurrentCardState))
  (bind (_value _returnvalue) (Utilities|Map|Find _materialmap _currentcardstate))
  (if _returnvalue
    (for (_array_element _array_index) (.materials _value)
      (Rendering|Material|SetMaterial (Variables|Default|GetCard%20Sleeve2) _array_index _array_element))))

(event EventTick
  (params (DeltaSeconds :type Float%20%28single-precision%29))
  (Transformation|AddLocalRotation (Variables|Default|GetPiece_Mesh) (Math|Rotator|MakeRotator 0.0 0.0 (* DeltaSeconds 36.0)) false false))

(event EventBPEonDrawCard
  (bind _cardrowhandle (Variables|Default|GetCardRowHandle))
  (bind (_datatable _rowname) (Utilities|Struct|BreakDataTableRowHandle _cardrowhandle))
  (bind _returnvalue (Utilities|GetDataTableRow _datatable _rowname)
    (:then
      (if (Utilities|Enum|Equal(Enum) (.EffectType (Utilities|Struct|BreakCardData _returnvalue)) "Gold")
        (Audio|PlaySoundatLocation (Variables|Default|GetSoundCue_DrawGold) (Transformation|GetActorLocation) "0, 0, 0" 1.0 1.0 0.0 0 0 0 0)
        (else
          (Audio|PlaySoundatLocation (Variables|Default|GetSoundCue_Draw) (Transformation|GetActorLocation) "0, 0, 0" 1.0 1.0 0.0 0 0 0 0))))))

(event EventBPEonPlay
  (params (IsMovement :type Boolean))
  (if IsMovement
    (Audio|PlaySound2D "/Game/Sounds/Cue/CUE-PlayMoveCard_Cue.CUE-PlayMoveCard_Cue" 1.0 1.0 0.0 0 0)
    (else
      (Audio|PlaySound2D "/Game/Sounds/Cue/CUE-PlayCard_Cue.CUE-PlayCard_Cue" 1.0 1.0 0.0 0 0))))

(fn ConstructionScript)