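; Card actor Blueprint that displays a Movement or Unit card with a rotating 3D piece, state feedback and sounds.
; ConstructCard uses row data to set the title, Movement sleeve or Unit pattern, then async-loads the piece mesh before setting the description and Gold gilding.
; UpdateMaterials maps card state to sleeve materials, while Tick spins the piece and sways the sleeve when hovered.
; BPE events play draw, discard, play, hover and select sounds.
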(event EventBPEonDiscardCard
  (Audio|PlaySoundatLocation (Variables|Default|GetSoundCue_Discard) (Transformation|GetActorLocation) "0, 0, 0" 1.0 1.0 0.0 0 0 0 0))

(event EventConstructCard
  (params (RowHandle :type Card%20Data%20Structure))
  (if (Utilities|Enum|Equal(Enum) (.cardtype RowHandle) "Movement")
    (Components|StaticMesh|SetStaticMesh (Variables|Default|GetCard%20Sleeve2) (Variables|Default|GetCardSleeveMovementMesh))
    (for (_array_element _array_index) (Variables|Default|GetMovementCardMaterialList)
      (Rendering|Material|SetMaterial (Variables|Default|GetCard%20Sleeve2) _array_index _array_element))
    (elif (Utilities|Enum|Equal(Enum) (.cardtype RowHandle) "Unit")
      (bind _asw_card_pattern_widget (Utilities|Casting|CastToW_CardPatternWidget (UserInterface|GetWidget (Variables|Default|GetPatternWidget))))
      (Default|SetPattern _asw_card_pattern_widget (.patterntexture RowHandle))))
  (bind _asw_card_title_widget (Utilities|Casting|CastToW_CardTitleWidget (UserInterface|GetWidget (Variables|Default|GetTitleWidget))))
  (Default|SetTitle _asw_card_title_widget (Utilities|Text|ToText(String) (.cardname RowHandle)))
  (bind _object (Utilities|AsyncLoadAsset (.cardunitstaticmesh RowHandle))
    (:Completed
      (bind _asstatic_mesh (Utilities|Casting|CastToStaticMesh _object))
      (Components|StaticMesh|SetStaticMesh (Variables|Default|GetPiece_Mesh) _asstatic_mesh)
      (bind _asw_card_pattern_widget_2 (Utilities|Casting|CastToW_CardPatternWidget (UserInterface|GetWidget (Variables|Default|GetPatternWidget)))
        (:then
          (Default|SetDescr _asw_card_pattern_widget_2 (Utilities|Text|ToText(String) (Utilities|String|ToString(Text) (.carddescription RowHandle)))))
        (:CastFailed
          _))
      (if (Utilities|Enum|Equal(Enum) (.effecttype RowHandle) "Gold")
        (Rendering|Material|SetMaterial (Variables|Default|GetCard%20Sleeve2) 0 "/Game/FBX/Cartes/Templates/Carte_Dorure.Carte_Dorure")))))

(event EventUpdateMaterials
  (bind _materialmap (Variables|Default|GetMaterialMap))
  (bind _currentcardstate (Variables|Default|GetCurrentCardState))
  (bind (_value _returnvalue) (Utilities|Map|Find _materialmap _currentcardstate))
  (if _returnvalue
    (for (_array_element _array_index) (.materials _value)
      (Rendering|Material|SetMaterial (Variables|Default|GetCard%20Sleeve2) _array_index _array_element))))

(event EventTick
  (params (DeltaSeconds :type Float%20%28single-precision%29))
  (Transformation|AddLocalRotation (Variables|Default|GetPiece_Mesh) (Math|Rotator|MakeRotator 0.0 0.0 (* DeltaSeconds 36.0)) false false)
  (if (Utilities|Enum|Equal(Enum) (Variables|Default|GetCurrentCardState) "Hovered")
    (Variables|Default|SetTimer (+ DeltaSeconds (Variables|Default|GetTimer)))
    (Transformation|SetRelativeRotation (Variables|Default|GetCard%20Sleeve2) (Math|Rotator|MakeRotator 0.0 0.0 (+ (* (* (- (Math|Trig|Sin(Radians) (Variables|Default|GetTimer)) 0.5) 3.6e+02) 0.04) 97.2)) false false)
    (else
      (Variables|Default|SetTimer 0.0)
      (Transformation|SetRelativeRotation (Variables|Default|GetCard%20Sleeve2) (Math|Rotator|MakeRotator 0.0 0.0 9e+01) false false))))

(event EventBPEonDrawCard
  (bind _cardrowhandle (Variables|Default|GetCardRowHandle))
  (bind (_datatable _rowname) (Utilities|Struct|BreakDataTableRowHandle _cardrowhandle))
  (bind _returnvalue (Utilities|GetDataTableRow _datatable _rowname)
    (:then
      (if (Utilities|Enum|Equal(Enum) (.EffectType (Utilities|Struct|BreakCardData _returnvalue)) "Gold")
        (Audio|PlaySoundatLocation (Variables|Default|GetSoundCue_DrawGold) (Transformation|GetActorLocation) "0, 0, 0" 1.0 1.0 0.0 0 0 0 0)
        (Variables|Default|SetBaseRotation (Variables|/Script/Engine.SceneComponent|GetRelativeRotation (Variables|Default|GetCCRootComponent)))
        (else
          (Audio|PlaySoundatLocation (Variables|Default|GetSoundCue_Draw) (Transformation|GetActorLocation) "0, 0, 0" 1.0 1.0 0.0 0 0 0 0))))))

(event EventBPEonPlay
  (params (IsMovement :type Boolean))
  (if IsMovement
    (Audio|PlaySound2D "/Game/Sounds/Cue/CUE-PlayMoveCard_Cue.CUE-PlayMoveCard_Cue" 1.0 1.0 0.0 0 0)
    (else
      (Audio|PlaySound2D "/Game/Sounds/Cue/CUE-PlayCard_Cue.CUE-PlayCard_Cue" 1.0 1.0 0.0 0 0))))

(event EventBPEHover
  (params (ToHover :type Boolean))
  (if ToHover
    (Audio|PlaySound2D "/Game/Sounds/SoundsAndre/Swipe.Swipe" 1.0 1.0 0.0 0 0)
    (else
      (Audio|PlaySound2D "/Game/Sounds/SoundsAndre/Click.Click" 1.0 1.0 0.0 0 0))))

(event EventBPESelect
  (params (ToSelect :type Boolean))
  (if ToSelect
    (Audio|PlaySound2D "/Game/Sounds/SoundsAndre/Switch.Switch" 1.0 1.0 0.0 0 0)
    (else
      (Audio|PlaySound2D "/Game/Sounds/SoundsAndre/Bloop.Bloop" 1.0 1.0 0.0 0 0))))

(fn ConstructionScript)