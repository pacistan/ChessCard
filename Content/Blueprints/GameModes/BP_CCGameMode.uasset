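; BP_CCGameMode is a game mode that holds the start of play until enough players have reported in through LoadingBackground.
; Each LoadingBackground call increments a counter and triggers StartPlayGame once the count reaches GetNumOfPlayersNeeded.
; StartPlayGame is guarded by a DoOnce, has BP_CCGameState remove the loading widget, then calls StartPlaySequence.
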(event Custom|LoadingBackground
  (bind _result (Math|Integer|IncrementInt (Variables|Default|GetloadingBackGroundPlayer))
    (:%20%20
      (bind _output_get (Variables|Default|SetloadingBackGroundPlayer _result))
      (if (>= _output_get (Class|CCGameMode|GetNumOfPlayersNeeded))
        (CallFunction|StartPlayGame)))))

(event Custom|StartPlayGame
  (Utilities|FlowControl|DoOnce false
    (:Completed
      (bind _asbp_ccgame_state (Utilities|Casting|CastToBP_CCGameState (Game|GetGameState)))
      (Default|RemoveLoadingWidget _asbp_ccgame_state)
      (Class|CCGameMode|StartPlaySequence))))

(fn ConstructionScript)