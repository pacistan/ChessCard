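; Game state for a turn-based card and piece game that drives phase music, sound cues and a loading widget.
; Game start plays planning and resolve tracks together, with resolve near-silent.
; On authority, state changes call MTC events that crossfade the tracks by volume and play new-turn or end-turn cues.
; Piece move ends trigger effect sounds for Embrasement and divine-anger Heracles, while separate events add or remove the loading widget.
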(event Custom|On%20Game%20State%20Change
  (params (CurrentState :type EGameState%20Enum :default "None"))
  (if (Ability|HasAuthority)
    (CallFunction|MTConGameStateChange CurrentState)))

(event Custom|MTC_OnGameStateChange
  (params (NewState :type EGameState%20Enum :default "None"))
  (if (and (Utilities|IsValid (Variables|Default|GetAC_PlanningPhaseMusic)) (Utilities|IsValid (Variables|Default|GetAC_ResolvePhaseMusic)))
    (switch Utilities|FlowControl|Switch|SwitchonEGameState NewState
      (:DrawingCards
        (Audio|PlaySound2D "/Game/Sounds/Cue/CUE-NewTurn_Cue.CUE-NewTurn_Cue" 1.0 1.0 0.0 0 0))
      (:Plannification
        (Audio|Components|Audio|AdjustVolume (Variables|Default|GetAC_PlanningPhaseMusic) (Variables|Default|GetMusicSwitchDuration) 1.0 "Linear" :!class /Script/Engine.AudioComponent)
        (Audio|Components|Audio|AdjustVolume (Variables|Default|GetAC_ResolvePhaseMusic) (Variables|Default|GetMusicSwitchDuration) 0.001 "Linear" :!class /Script/Engine.AudioComponent))
      (:Resolve
        (Audio|PlaySound2D "/Game/Sounds/Cue/CUE-EndTurn_Cue.CUE-EndTurn_Cue" 1.0 1.0 0.0 0 0)
        (Audio|Components|Audio|AdjustVolume (Variables|Default|GetAC_PlanningPhaseMusic) (Variables|Default|GetMusicSwitchDuration) 0.001 "Linear" :!class /Script/Engine.AudioComponent)
        (Audio|Components|Audio|AdjustVolume (Variables|Default|GetAC_ResolvePhaseMusic) (Variables|Default|GetMusicSwitchDuration) 1.0 "Linear" :!class /Script/Engine.AudioComponent)))
    (else
      (Development|PrintString "Audio Cue not valid"))))

(event Custom|MTC_OnPieceMoveEnd
  (params (EffectType :type EEffectType%20Enum :default "Midas") (IsDivineAnger :type Boolean))
  (switch Utilities|FlowControl|Switch|SwitchonEEffectType EffectType
    (:Heracles
      (if IsDivineAnger
        (Audio|PlaySound2D "/Game/Sounds/Cue/CUE-MultimoveHeracles_Cue.CUE-MultimoveHeracles_Cue" 1.0 1.0 0.0 0 0)))
    (:Embrasement
      (Audio|PlaySound2D "/Game/Sounds/Cue/CUE-Explosion_Cue.CUE-Explosion_Cue" 1.0 1.0 0.0 0 0))))

(event Custom|AddLoadingWidget
  (Class|CCBPFunctionLibrary|AddWidgettoViewport (Game|GetGameInstance) (Variables|Default|GetLoadingWidget) 5))

(event Custom|RemoveLoadingWidget
  (Class|CCBPFunctionLibrary|RemoveWidgetfromViewport (Game|GetGameInstance) (Variables|Default|GetLoadingWidget)))

(event EventBPEStartGame
  (bind _returnvalue (Audio|CreateSound2D (Variables|Default|GetPlanningPhaseMusic) 1.0 1.0 0.0 0))
  (bind _output_get (Variables|Default|SetAC_PlanningPhaseMusic _returnvalue))
  (Class|CCGameState|BPCRegisterAudioComponent _output_get)
  (Audio|Components|Audio|Play _output_get 0.0)
  (bind _returnvalue_2 (Audio|CreateSound2D (Variables|Default|GetResolvePhaseMusic) 1.0 1.0 0.0 0))
  (bind _output_get_2 (Variables|Default|SetAC_ResolvePhaseMusic _returnvalue_2))
  (Components|Activation|Activate _output_get_2 false)
  (Class|CCGameState|BPCRegisterAudioComponent _output_get_2)
  (Audio|Components|Audio|Play _output_get_2 0.0)
  (Audio|Components|Audio|AdjustVolume _output_get_2 0.0 0.001 "Linear" :!class /Script/Engine.AudioComponent))

(event EventBPEonPieceEndMove
  (params (EffectType :type EEffectType%20Enum :default "Midas") (IsDivineAnger :type Boolean))
  (CallFunction|MTConPieceMoveEnd EffectType IsDivineAnger))

(event EventBeginPlay
  (EventDispatchers|BindEventtoOnGameStateChange (delegate Custom|On%20Game%20State%20Change)))

(fn ConstructionScript)