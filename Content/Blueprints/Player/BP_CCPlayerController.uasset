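; Player controller that streams in a background level for the local player and notifies the game mode when it is ready.
; LoadingBackground loads the soft-referenced BackGroundToLoad level as an instance at the given PlayerStart's location and rotation.
; The instance's loaded callback triggers BackGroundIsLoad, which calls LoadingBackground on BP_CCGameMode.
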(event Custom|OnLevelLoad
  (CallFunction|BackGroundIsLoad))

(event Custom|LoadingBackground
  (params (PlayerStart :type Player%20Start%20Object%20Reference))
  (bind _back_ground_to_load (Variables|Default|GetBack%20Ground%20to%20Load))
  (Development|PrintText "Load backGround")
  (if (Pawn|IsLocalPlayerController)
    (if (Utilities|IsValidSoftObjectReference _back_ground_to_load)
      (bind (_boutsuccess _returnvalue) (Class|LevelStreamingDynamic|LoadLevelInstancebySoftObjectPtr _back_ground_to_load (Transformation|GetActorLocation PlayerStart) (Transformation|GetActorRotation PlayerStart) "" 0 false))
      (if _boutsuccess
        (EventDispatchers|BindEventtoOnLevelLoaded _returnvalue (delegate Custom|OnLevelLoad))
        (else
          (Development|PrintString "Level instance load failed"))))))

(event Custom|BackGroundIsLoad
  (bind _asbp_ccgame_mode (Utilities|Casting|CastToBP_CCGameMode (Game|GetGameMode)))
  (Default|LoadingBackground _asbp_ccgame_mode))

(fn ConstructionScript)