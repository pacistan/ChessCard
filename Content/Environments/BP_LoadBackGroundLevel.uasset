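; BP_LoadBackGroundLevel is a placeable actor that streams in a background level as a level instance.
; On BeginPlay, if enabled and the level soft reference is valid, it loads that level at the actor's own location and rotation.
; A successful load binds the level-loaded callback, which is currently empty; a failed load prints an error message.
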(event Custom|OnLevelLoad)

(event EventBeginPlay
  (bind _backgroundtoload (Variables|Default|GetBackGroundToLoad))
  (if (Variables|Default|GetShouldLoadBackGround)
    (if (Utilities|IsValidSoftObjectReference _backgroundtoload)
      (bind (_boutsuccess _returnvalue) (Class|LevelStreamingDynamic|LoadLevelInstancebySoftObjectPtr _backgroundtoload (Transformation|GetActorLocation) (Transformation|GetActorRotation) "" 0 false))
      (if _boutsuccess
        (EventDispatchers|BindEventtoOnLevelLoaded _returnvalue (delegate Custom|OnLevelLoad))
        (else
          (Development|PrintString "Level instance load failed"))))))

(fn ConstructionScript)